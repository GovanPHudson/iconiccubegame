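; Crane puzzle output, an unfinished autosaved draft meant to rotate when activated.
; Activated and Deactivated set a ShouldRotate flag, which starts off through a Deactivated call on BeginPlay.
; Tick loops on that flag with only debug prints, so activation causes an endless loop as nothing inside clears it.
; The timeline and relative-rotation nodes are unwired, so the crane never actually turns.
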(event `self.ReceiveBeginPlay`
  (`parent.ReceiveBeginPlay`)
  (`self.Deactivated`))

(event `self.ReceiveTick`
  (params (DeltaSeconds :type "Float (single-precision)"))
  (`parent.ReceiveTick` DeltaSeconds)
  (while (`self.ShouldRotate?`)
    (`KismetSystemLibrary.PrintString` "Hello" true false))
  (`KismetSystemLibrary.PrintString` "DONE BOI"))

(event `self.Activated`
  (set `self.ShouldRotate?` true))

(event `self.Deactivated`
  (set `self.ShouldRotate?` false))

(fn `UserConstructionScript`
  (`parent.UserConstructionScript`))