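; Spinner gear puzzle input that the player activates by hitting it with Cubie's spin attack.
; While active, damage from a Cubie character checks the player character's spin-attack state.
; A spinning hit rotates the gear a small step and switches its input on, while any other hit counts as a punch and only prints a debug message.
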(event `self.ReceiveAnyDamage`
  (params (Damage :type "Float (single-precision)") (DamageType :type "DamageType Object Reference") (InstigatedBy :type "Controller Object Reference") (DamageCauser :type "Actor Object Reference"))
  (if (and (`KismetArrayLibrary.Array_Contains` (`|MakeArray` "/Game/IconicCubeGame/Cubie/Blueprints/BP_Cubie_Character.BP_Cubie_Character_C" :!type "Actor Class Reference") (`GameplayStatics.GetObjectClass` DamageCauser)) (`self.Active`))
    (bind _asbp_cubie_character (cast `/Game/IconicCubeGame/Cubie/Blueprints/BP_Cubie_Character` (`GameplayStatics.GetPlayerCharacter` 0)))
    (if (`/Game/IconicCubeGame/Cubie/Blueprints/BP_Cubie_Character.AttackSpinning?` _asbp_cubie_character)
      (`self.Is Currently Being Spun`)
      (else
        (`self.Is Currently Being Punched`)))))

(event `Is Currently Being Spun`
  (`KismetSystemLibrary.PrintString` "Hello")
  (`self.K2_AddActorLocalRotation` (struct :`Yaw` 4.0))
  (`self.Set Input On`))

(event `Is Currently Being Punched`
  (`KismetSystemLibrary.PrintString` "Wrong move idiot"))

(fn `UserConstructionScript`
  (`parent.UserConstructionScript`))