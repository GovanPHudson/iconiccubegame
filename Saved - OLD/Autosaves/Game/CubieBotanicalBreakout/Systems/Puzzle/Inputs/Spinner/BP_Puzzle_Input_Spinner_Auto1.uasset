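; BP_Puzzle_Input_Spinner is an early stub of a puzzle input meant to respond to Cubie's spin attack.
; When Active and damaged by a BP_Cubie_Character, it checks the player character's AttackSpinning flag to tell a spin from a punch.
; Each case fires its own custom event, which so far only prints a debug string.
; Tick checks Active but does nothing yet.
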(event `self.ReceiveAnyDamage`
  (params (Damage :type "Float (single-precision)") (DamageType :type "DamageType Object Reference") (InstigatedBy :type "Controller Object Reference") (DamageCauser :type "Actor Object Reference"))
  (if (and (`KismetArrayLibrary.Array_Contains` (`|MakeArray` "/Game/IconicCubeGame/Cubie/Blueprints/BP_Cubie_Character.BP_Cubie_Character_C" :!type "Actor Class Reference") (`GameplayStatics.GetObjectClass` DamageCauser)) (`self.Active`))
    (bind _asbp_cubie_character (cast `/Game/IconicCubeGame/Cubie/Blueprints/BP_Cubie_Character` (`GameplayStatics.GetPlayerCharacter` 0)))
    (if (`/Game/IconicCubeGame/Cubie/Blueprints/BP_Cubie_Character.AttackSpinning?` _asbp_cubie_character)
      (`self.Is currently being spun`)
      (else
        (`self.Is currently bring punched`)))))

(event `Is currently being spun`
  (`KismetSystemLibrary.PrintString` "Hello"))

(event `self.ReceiveTick`
  (params (DeltaSeconds :type "Float (single-precision)"))
  (`parent.ReceiveTick` DeltaSeconds)
  (if (`self.Active`)
    _))

(event `Is currently bring punched`
  (`KismetSystemLibrary.PrintString` "Wrong move idiot"))

(fn `UserConstructionScript`)