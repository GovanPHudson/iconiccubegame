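; Spinner gear puzzle input that Cubie turns on with a sustained spin attack.
; While active, spin-attack damage rotates the gear, plays a sound and sets BeingSpun, which Tick uses to count down SpinningTIMER before clearing it through a delay.
; A spin hit at zero timer calls SetInputOn.
; Other non-charging attacks play a throttled metal clang, with debug prints throughout.
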(event `self.ReceiveAnyDamage`
  (params (Damage :type "Float (single-precision)") (DamageType :type "DamageType Object Reference") (InstigatedBy :type "Controller Object Reference") (DamageCauser :type "Actor Object Reference"))
  (if (and (`KismetArrayLibrary.Array_Contains` (`|MakeArray` "/Game/IconicCubeGame/Cubie/Blueprints/BP_Cubie_Character.BP_Cubie_Character_C" :!type "Actor Class Reference") (`GameplayStatics.GetObjectClass` DamageCauser)) (`self.Active`))
    (bind _asbp_cubie_character (cast `/Game/IconicCubeGame/Cubie/Blueprints/BP_Cubie_Character` (`GameplayStatics.GetPlayerCharacter` 0)))
    (if (`/Game/IconicCubeGame/Cubie/Blueprints/BP_Cubie_Character.AttackSpinning?` _asbp_cubie_character)
      (bind _output_get (set `self.Being Spun?` true))
      (if _output_get
        (`self.K2_AddActorLocalRotation` (struct :`Yaw` 4.0))
        (`GameplayStatics.PlaySoundAtLocation` "/Game/IconicCubeGame/Cubie/Audio/A_Cubie_CDPlayer.A_Cubie_CDPlayer" (`self.K2_GetActorLocation`) (struct) 1.0 1.0 0.0 null null null)
        (if (<= (`self.Spinning TIMER`) 0.0)
          (`self.Spun Long Enough?`)))
      (else
        (`self.Is Currently Being Punched`)))))

(event `Spun Long Enough?`
  (`KismetSystemLibrary.PrintString` "Hello")
  (`self.Set Input On`))

(event `self.ReceiveTick`
  (params (DeltaSeconds :type "Float (single-precision)"))
  (if (`self.Active?`)
    (if (`self.Being Spun?`)
      (bind _output_get (set `self.Spinning TIMER` (`KismetMathLibrary.FClamp` (- (`self.Spinning TIMER`) (`GameplayStatics.GetWorldDeltaSeconds`)) 0.0 (`self.Spinning TIMER`))))
      (`KismetSystemLibrary.PrintString` (`KismetStringLibrary.Conv_DoubleToString` _output_get))
      (`KismetSystemLibrary.Delay` 2.0)
      (set `self.Being Spun?` false))))

(event `Is Currently Being Punched`
  (if (not (`/Game/IconicCubeGame/Cubie/Blueprints/BP_Cubie_Character.AttackCharging?` (stale `self.ReceiveAnyDamage` _asbp_cubie_character)))
    (`/Engine/EditorBlueprintResources/StandardMacros.DoOnce` false :!label _label
      (:`Completed`
        (`GameplayStatics.PlaySoundAtLocation` "/Game/IconicCubeGame/Audio/FinalAudio/SFX/A_Metal_Clang_01_Cue.A_Metal_Clang_01_Cue" (`self.K2_GetActorLocation`) (struct) 1.0 1.0 0.0 null null null)
        (`KismetSystemLibrary.PrintString` "Wrong move idiot")
        (`KismetSystemLibrary.Delay` 0.5)
        (goto _label :!via `Reset`)))))

(fn `UserConstructionScript`
  (`parent.UserConstructionScript`))