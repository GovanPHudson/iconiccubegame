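; Teleport pad hazard that sends player 0's pawn to DestLocation after about two seconds of standing on it.
; Overlap lights the pad and starts energy effects, a Tick countdown and a matching Delay, with no check on the overlapping actor.
; An expired countdown teleports with arrival effects; otherwise the pad sparks and briefly deactivates.
; Stepping off pauses the countdown and darkens the pad; StepOffCOOLDOWN is set but never read.
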(event `self.ReceiveActorBeginOverlap`
  (params (OtherActor :type "Actor Object Reference"))
  (bind _returnvalue (`self.K2_GetActorLocation`))
  (bind _dest_location (`self.Dest Location`))
  (if (`self.Pad Active?`)
    (set `self.Stood On?` true)
    (set `self.Stand On TIMER` 2.0)
    (`PrimitiveComponent.SetMaterial` (`self.SM_Prop_Log_Slice_Large`) 0 "/Game/CubieBotanicalBreakout/Seamless/Metal/MI_Seamless_Metal_Hex_Light.MI_Seamless_Metal_Hex_Light")
    (`ActorComponent.Activate` (`self.NS_Energy`) false)
    (`GameplayStatics.PlaySoundAtLocation` "/Game/IconicCubeGame/Sequences/Audio/ZapLong.ZapLong" _returnvalue (struct) 3.0 1.0 0.0 null null null)
    (if (`self.Stood On?`)
      (`KismetSystemLibrary.Delay` 2.0)
      (if (<= (`self.Stand On TIMER`) 0.0)
        (`GameplayStatics.PlaySoundAtLocation` "/Game/IconicCubeGame/Sequences/Audio/ZapDeepShort.ZapDeepShort" _dest_location (struct) 3.0 1.0 0.0 null null null)
        (`GameplayStatics.PlaySoundAtLocation` "/Game/CubieBotanicalBreakout/Hazards/Electric/A_Hazard_Electric_Zap.A_Hazard_Electric_Zap" _dest_location (struct) 4.0 1.0 0.0 null null null)
        (`GameplayStatics.PlaySoundAtLocation` "/Game/IconicCubeGame/Audio/FinalAudio/SFX/A_SmallExplosion_02.A_SmallExplosion_02" _dest_location (struct) 1.0 1.0 0.0 null null null)
        (`self.K2_TeleportTo` :`self` (`Controller.K2_GetPawn` (`GameplayStatics.GetPlayerController` 0)) :`DestLocation` (`self.Dest Location`))
        (`NiagaraFunctionLibrary.SpawnSystemAtLocation` "/Game/RetroParticles/Particles/Systems/NS_Energy_Out.NS_Energy_Out" (`self.Dest Location`))
        (else
          (`GameplayStatics.PlaySoundAtLocation` "/Game/IconicCubeGame/Sequences/Audio/PowerDownBC.PowerDownBC" _returnvalue (struct) 1.0 2.0 0.0 null null null)
          (`ActorComponent.Activate` (`self.NS_Sparks_02`) false)
          (`ActorComponent.Deactivate` (`self.NS_Electricity`))
          (set `self.Pad Active?` false)
          (`KismetSystemLibrary.Delay` 2.0)
          (set `self.Pad Active?` true))))))

(event `self.ReceiveActorEndOverlap`
  (params (OtherActor :type "Actor Object Reference"))
  (set `self.Stood On?` false)
  (`PrimitiveComponent.SetMaterial` (`self.SM_Prop_Log_Slice_Large`) 0 "/Game/CubieBotanicalBreakout/Seamless/Metal/MI_Seamless_Metal_Hex_Dark.MI_Seamless_Metal_Hex_Dark")
  (`ActorComponent.Deactivate` (`self.NS_Energy`))
  (set `self.Step Off COOLDOWN` 2.0)
  (`KismetSystemLibrary.PrintString` "Player Stepped Off"))

(event `self.ReceiveTick`
  (params (DeltaSeconds :type "Float (single-precision)"))
  ;[1 1 1] Stand On Timer
  (if (`self.Stood On?`)
    (bind _output_get (set `self.Stand On TIMER` (`KismetMathLibrary.FClamp` (- (`self.Stand On TIMER`) (`GameplayStatics.GetWorldDeltaSeconds`)) 0.0 (`self.Stand On TIMER`))))
    (`KismetSystemLibrary.PrintString` (`KismetStringLibrary.Conv_DoubleToString` _output_get))))

(fn `UserConstructionScript`)